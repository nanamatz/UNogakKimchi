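; Player character Blueprint that handles a directional tumble (dodge roll) and experience gain.
; Tumble input, blocked while tumbling, attacking or skill casting, picks a montage from movement axes: backward input overrides sideways, and no input rolls forward.
; Each direction's timeline scales MoveDistance to overwrite horizontal velocity along the actor's axes, preserving Z.
; AddExp adds to the Stat total and prints the previous value.
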(event `AddExp`
  (params (Exp :type Integer))
  (bind _stat (`self.Stat`))
  (bind _returnvalue (`MyStatComponent.GetExp` _stat))
  (`MyStatComponent.SetExp` _stat (+ Exp _returnvalue))
  (`KismetSystemLibrary.PrintString` (`KismetStringLibrary.Conv_IntToString` _returnvalue)))

(event `InputAction|Tumble`
  (params (Key :type "Key Structure"))
  (bind (_velocity_x _velocity_y _velocity_z) (`KismetMathLibrary.BreakVector` (`MovementComponent.Velocity` (`self.CharacterMovement`))))
  (bind (_velocity_x_2 _velocity_y_2 _velocity_z_2) (`KismetMathLibrary.BreakVector` (`MovementComponent.Velocity` (`self.CharacterMovement`))))
  (bind (_velocity_x_3 _velocity_y_3 _velocity_z_3) (`KismetMathLibrary.BreakVector` (`MovementComponent.Velocity` (`self.CharacterMovement`))))
  (bind (_velocity_x_4 _velocity_y_4 _velocity_z_4) (`KismetMathLibrary.BreakVector` (`MovementComponent.Velocity` (`self.CharacterMovement`))))
  (:`Pressed`
    (if (and (not (`self.IsTumbling`)) (not (`self.IsAttacking`)) (not (`self.IsSkillCasting`)))
      (set `self.vertical` (`self.GetInputAxisValue`))
      (set `self.horizontal` (`self.GetInputAxisValue`))
      (`self.Tumble`)
      (if (>= (`self.vertical`) 0.0)
        (if (>= (`self.horizontal`) 0.0)
          (if (== (`self.horizontal`) 0.0)
            ;[1 1 1] FrontTumble
            (`|PlayMontage` (`self.Mesh`) "/Game/Animations/BP_TumbleMontage.BP_TumbleMontage"
              (:`then`
                (bind (_direction _distancemultiplier) (`Timeline|타임라인_1` :!via `PlayFromStart`)
                  (:`Update`
                    (bind (_returnvalue_x _returnvalue_y) (`KismetMathLibrary.BreakVector` (* (`self.GetActorForwardVector`) (* _distancemultiplier (`self.MoveDistance`)))))
                    (set `MovementComponent.Velocity` (`KismetMathLibrary.MakeVector` _returnvalue_x _returnvalue_y _velocity_z) (`self.CharacterMovement`))))))
            (else
              ;[1 1 1] RightTumble
              (`|PlayMontage` (`self.Mesh`) "/Game/Animations/BP_TumbleRightMontage.BP_TumbleRightMontage"
                (:`then`
                  (bind (_direction_2 _distancemultiplier_2) (`Timeline|타임라인_3` :!via `PlayFromStart`)
                    (:`Update`
                      (bind (_returnvalue_x_2 _returnvalue_y_2) (`KismetMathLibrary.BreakVector` (* (`self.GetActorRightVector`) (* _distancemultiplier_2 (`self.MoveDistance`)))))
                      (set `MovementComponent.Velocity` (`KismetMathLibrary.MakeVector` _returnvalue_x_2 _returnvalue_y_2 _velocity_z_4) (`self.CharacterMovement`))))))))
          (else
            ;[1 1 1] LeftTumble
            (`|PlayMontage` (`self.Mesh`) "/Game/Animations/BP_TumbleLeftMontage.BP_TumbleLeftMontage"
              (:`then`
                (bind (_direction_3 _distancemultiplier_3) (`Timeline|타임라인_0` :!via `PlayFromStart`)
                  (:`Update`
                    (bind (_returnvalue_x_3 _returnvalue_y_3) (`KismetMathLibrary.BreakVector` (* (`self.GetActorRightVector`) (* _distancemultiplier_3 (`self.MoveDistance`) -1.0))))
                    (set `MovementComponent.Velocity` (`KismetMathLibrary.MakeVector` _returnvalue_x_3 _returnvalue_y_3 _velocity_z_2) (`self.CharacterMovement`))))))))
        (else
          ;[1 1 1] RearTumble
          (`|PlayMontage` (`self.Mesh`) "/Game/Animations/BP_TumbleBackMontage.BP_TumbleBackMontage"
            (:`then`
              (bind (_direction_4 _distancemultiplier_4) (`Timeline|타임라인_2` :!via `PlayFromStart`)
                (:`Update`
                  (bind (_returnvalue_x_4 _returnvalue_y_4) (`KismetMathLibrary.BreakVector` (* (`self.GetActorForwardVector`) (* _distancemultiplier_4 (`self.MoveDistance`) -1.0))))
                  (set `MovementComponent.Velocity` (`KismetMathLibrary.MakeVector` _returnvalue_x_4 _returnvalue_y_4 _velocity_z_3) (`self.CharacterMovement`)))))))))))

(fn `UserConstructionScript`)