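; AI controller for the boss enemy that runs its behavior tree on possess and keeps its blackboard updated.
; Sight perception sets the player as the target, and a timer clears it after line of sight is lost.
; Each tick it copies the boss's death state and compares player distance to set attack and dash flags, rolling a random number while in attack range.
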(event `self.ReceiveTick`
  (params (DeltaSeconds :type "Float (single-precision)"))
  (bind _asbp_my_boss (cast `/Game/MyBoss/BluePrint/BP_MyBoss` (`BlackboardComponent.GetValueAsObject` (`self.Blackboard`) (`self.SelfActor`))))
  (`BlackboardComponent.SetValueAsBool` (`self.Blackboard`) (`self.IsDie`) (`MyBossClass.isDie` _asbp_my_boss)) ; 죽었는지 확인
  ;[1 1 1] Tick마다 보스와 플레이어 사이 거리 구해서 BB업데이트
  (bind _asbp_my_boss_2 (cast `/Game/MyBoss/BluePrint/BP_MyBoss` (`BlackboardComponent.GetValueAsObject` (`self.Blackboard`) (`self.SelfActor`))))
  (bind _asmy_character (cast `MyCharacter` (`BlackboardComponent.GetValueAsObject` (`self.Blackboard`) (`self.EnemyActor`))))
  (`|ExecutionSequence`
    (:`then_0`
      (bind _returnvalue (`self.GetDistanceTo` _asbp_my_boss_2 _asmy_character))
      (if (<= _returnvalue (`MyBossClass.AttackRange` _asbp_my_boss_2))
        (`BlackboardComponent.SetValueAsBool` (`self.Blackboard`) (`self.IsAttack`) true) ; 사거리 안에 들어옴
        (`BlackboardComponent.SetValueAsInt` (`self.Blackboard`) (`self.CreateRandomNumber`) (`KismetMathLibrary.RandomInteger` 100))
        (else
          (`BlackboardComponent.SetValueAsBool` (`self.Blackboard`) (`self.IsAttack`) false) ; 사거리 밖임
        )))
    (:`then_1`
      (if (>= _returnvalue 1000.0)
        (`BlackboardComponent.SetValueAsBool` (`self.Blackboard`) (`self.CanDash`) true) ; 사거리 안에 들어옴
        (else
          (`BlackboardComponent.SetValueAsBool` (`self.Blackboard`) (`self.CanDash`) false) ; 사거리 안에 들어옴
        )))))

(event `self.ReceiveBeginPlay`
  ;[1 1 1] BossCharacter 변수 가져오기
  (cast `/Game/MyBoss/BluePrint/BP_MyBoss` (`BlackboardComponent.GetValueAsObject` (`self.Blackboard`) (`self.SelfActor`)))
  (set `self.Boss_Character` null))

(event `self.ReceivePossess`
  (params (PossessedPawn :type "Pawn Object Reference"))
  ;[1 1 1] Behavior Tree 실행
  (`self.RunBehaviorTree` "/Game/MyBoss/BehaviorTree/BT_MyBoss.BT_MyBoss"))

(event `self.AIPerception.OnTargetPerceptionUpdated`
  (params (Actor :type "Actor Object Reference") (Stimulus :type "AIStimulus Structure"))
  (bind _blackboard (`self.Blackboard`))
  ;[1 1 1] 시야 안에 들어왔을 때 BB값 업데이트
  (if (and (`self.ActorHasTag` Actor "Player") (`.bSuccessfullySensed` (break `AIStimulus` Stimulus)))
    (`KismetSystemLibrary.K2_ClearAndInvalidateTimerHandle` (`self.EnemyTimer`))
    (`BlackboardComponent.SetValueAsBool` _blackboard (`self.HasLineOfSight`) true)
    (`BlackboardComponent.SetValueAsObject` _blackboard (`self.EnemyActor`) Actor)
    (else
      (bind _returnvalue (`KismetSystemLibrary.K2_SetTimerDelegate` (delegate `StartEnemyTimer`) (`self.LineOfSightTime`)))
      (set `self.EnemyTimer` _returnvalue))))

(event `StartEnemyTimer`
  (bind _blackboard (`self.Blackboard`))
  ;[1 1 1] 시야 안에 들어왔을 때 BB값 업데이트
  (`BlackboardComponent.SetValueAsBool` _blackboard (`self.HasLineOfSight`) false)
  (`BlackboardComponent.SetValueAsObject` _blackboard (`self.EnemyActor`) null))

(fn `UserConstructionScript`)